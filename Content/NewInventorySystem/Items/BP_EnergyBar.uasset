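; BP_EnergyBar is an energy bar item in the new inventory system, derived from a parent item Blueprint that supplies its behavior.
; UseItem and the construction script defer to the parent, and SetMaterial calls the parent with EnabledFOV forced to false.
; The animation, timeline, montage-callback and SRV_FinishEat events have empty bodies here, so this file adds no eating or energy logic of its own.
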(event Custom|Timeline_0__FinishedFunc)

(event Custom|Timeline_0__UpdateFunc)

(event Custom|OnBlendOut_AE2A3D66458122E1C7ABE08F22ADD52E
  (params (NotifyName :type Name)))

(event Custom|OnCompleted_AE2A3D66458122E1C7ABE08F22ADD52E
  (params (NotifyName :type Name)))

(event Custom|PlayAnimation)

(event Custom|SRV_FinishEat)

(event Custom|OnNotifyEnd_2EF3CB7C458DDF5DC53EA4A7CA6DA62A
  (params (NotifyName :type Name)))

(event Custom|OnNotifyBegin_2EF3CB7C458DDF5DC53EA4A7CA6DA62A
  (params (NotifyName :type Name)))

(event Custom|OnInterrupted_2EF3CB7C458DDF5DC53EA4A7CA6DA62A
  (params (NotifyName :type Name)))

(event Custom|OnBlendOut_2EF3CB7C458DDF5DC53EA4A7CA6DA62A
  (params (NotifyName :type Name)))

(event Custom|OnCompleted_2EF3CB7C458DDF5DC53EA4A7CA6DA62A
  (params (NotifyName :type Name)))

(event Custom|OnNotifyEnd_AE2A3D66458122E1C7ABE08F22ADD52E
  (params (NotifyName :type Name)))

(event Custom|OnNotifyBegin_AE2A3D66458122E1C7ABE08F22ADD52E
  (params (NotifyName :type Name)))

(event Custom|OnInterrupted_AE2A3D66458122E1C7ABE08F22ADD52E
  (params (NotifyName :type Name)))

(event EventBeginPlay
  (|CallParentFunction) ; 此节点被禁用，将不会被调用。\n从引脚连出引线来编译功能。
)

(event Collision|EventActorBeginOverlap
  (params (OtherActor :type Actor%20Object%20Reference))
  (|CallParentFunction OtherActor) ; 此节点被禁用，将不会被调用。\n从引脚连出引线来编译功能。
)

(event EventTick
  (params (DeltaSeconds :type Float%20%28single-precision%29))
  (|CallParentFunction DeltaSeconds) ; 此节点被禁用，将不会被调用。\n从引脚连出引线来编译功能。
)

(event EventUseItem
  (|CallParentFunction))

(fn ConstructionScript
  (|CallParentFunction))

(fn SetMaterial
  (params (EnabledFOV :type Boolean))
  (|CallParentFunction false))