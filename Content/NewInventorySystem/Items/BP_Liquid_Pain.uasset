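; BP_Liquid_Pain is an inventory item Blueprint, by its name a pain-related liquid variant of a parent item class.
; UseItem, SetMaterial and the construction script only forward to the parent.
; PlayAnimation, SRV_FinishDrink, the montage callbacks and the timeline events have empty bodies, and BeginPlay, Tick and overlap are disabled stubs, so the graphs add no pain-specific logic.
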(event Custom|Timeline_0__FinishedFunc)

(event Custom|Timeline_0__UpdateFunc)

(event Custom|OnNotifyEnd_0F271FAE4B4291EFCF443CB4D7BCBFE5
  (params (NotifyName :type Name)))

(event Custom|OnNotifyBegin_0F271FAE4B4291EFCF443CB4D7BCBFE5
  (params (NotifyName :type Name)))

(event Custom|OnInterrupted_0F271FAE4B4291EFCF443CB4D7BCBFE5
  (params (NotifyName :type Name)))

(event Custom|OnBlendOut_0F271FAE4B4291EFCF443CB4D7BCBFE5
  (params (NotifyName :type Name)))

(event Custom|OnCompleted_0F271FAE4B4291EFCF443CB4D7BCBFE5
  (params (NotifyName :type Name)))

(event Custom|PlayAnimation)

(event Custom|SRV_FinishDrink)

(event EventBeginPlay
  (|CallParentFunction) ; 此节点被禁用，将不会被调用。\n从引脚连出引线来编译功能。
)

(event Collision|EventActorBeginOverlap
  (params (OtherActor :type Actor%20Object%20Reference))
  (|CallParentFunction OtherActor) ; 此节点被禁用，将不会被调用。\n从引脚连出引线来编译功能。
)

(event EventTick
  (params (DeltaSeconds :type Float%20%28single-precision%29))
  (|CallParentFunction DeltaSeconds) ; 此节点被禁用，将不会被调用。\n从引脚连出引线来编译功能。
)

(event EventUseItem
  (|CallParentFunction))

(fn ConstructionScript
  (|CallParentFunction))

(fn SetMaterial
  (params (EnabledFOV :type Boolean))
  (|CallParentFunction EnabledFOV))