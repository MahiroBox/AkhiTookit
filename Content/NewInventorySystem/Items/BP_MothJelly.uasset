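; BP_MothJelly is an item Blueprint in the new inventory system, apparently an edible consumable, with no logic of its own in its graphs.
; UseItem, ToggleEvent, OnEventLoaded and the construction script only call their parent versions.
; The HoverDown timeline, montage callbacks, PlayAnimation and SRV_FinishEat are empty stubs, so any working behavior comes from the parent class.
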(event Custom|HoverDown__FinishedFunc)

(event Custom|HoverDown__UpdateFunc)

(event Custom|OnNotifyEnd_1CCDCF174099237E391B5AA1C23BF140
  (params (NotifyName :type Name)))

(event Custom|OnNotifyBegin_1CCDCF174099237E391B5AA1C23BF140
  (params (NotifyName :type Name)))

(event Custom|OnInterrupted_1CCDCF174099237E391B5AA1C23BF140
  (params (NotifyName :type Name)))

(event Custom|OnBlendOut_1CCDCF174099237E391B5AA1C23BF140
  (params (NotifyName :type Name)))

(event Custom|OnCompleted_1CCDCF174099237E391B5AA1C23BF140
  (params (NotifyName :type Name)))

(event Custom|PlayAnimation)

(event Custom|SRV_FinishEat)

(event EventBeginPlay
  (|CallParentFunction) ; 此节点被禁用，将不会被调用。\n从引脚连出引线来编译功能。
)

(event Collision|EventActorBeginOverlap
  (params (OtherActor :type Actor%20Object%20Reference))
  (|CallParentFunction OtherActor) ; 此节点被禁用，将不会被调用。\n从引脚连出引线来编译功能。
)

(event EventTick
  (params (DeltaSeconds :type Float%20%28single-precision%29))
  (|CallParentFunction DeltaSeconds) ; 此节点被禁用，将不会被调用。\n从引脚连出引线来编译功能。
)

(event EventUseItem
  (|CallParentFunction))

(event EventToggleEvent
  (params (Enable :type Boolean))
  (|CallParentFunction Enable))

(event EventOnEventLoaded
  (params (EventType :type Byte :default 0))
  (|CallParentFunction EventType))

(fn ConstructionScript
  (|CallParentFunction))