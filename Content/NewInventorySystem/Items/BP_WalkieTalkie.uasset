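; Walkie-talkie item for the inventory system, currently a skeleton with no radio behavior of its own.
; BeginPlay, Destroyed, UseItem, construction and SetMaterial only forward to the parent item class.
; Radio activation, connect and alarm events, alarm reset and the NumConnected RepNotify are empty stubs.
; Two sets of montage notify and completion callbacks are also empty.
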(event Custom|OnNotifyEnd_0A19368B42B332B8561A4A9702E5897B
  (params (NotifyName :type Name)))

(event Custom|OnNotifyBegin_0A19368B42B332B8561A4A9702E5897B
  (params (NotifyName :type Name)))

(event Custom|MC_Connect)

(event Custom|MC_Alarm)

(event Custom|OnInterrupted_0A19368B42B332B8561A4A9702E5897B
  (params (NotifyName :type Name)))

(event Custom|OnBlendOut_0A19368B42B332B8561A4A9702E5897B
  (params (NotifyName :type Name)))

(event Custom|OnCompleted_0A19368B42B332B8561A4A9702E5897B
  (params (NotifyName :type Name)))

(event Custom|OnNotifyEnd_F5534A844701AD21AB1B749705B92259
  (params (NotifyName :type Name)))

(event Custom|OnNotifyBegin_F5534A844701AD21AB1B749705B92259
  (params (NotifyName :type Name)))

(event Custom|OnInterrupted_F5534A844701AD21AB1B749705B92259
  (params (NotifyName :type Name)))

(event Custom|OnBlendOut_F5534A844701AD21AB1B749705B92259
  (params (NotifyName :type Name)))

(event Custom|OnCompleted_F5534A844701AD21AB1B749705B92259
  (params (NotifyName :type Name)))

(event EventBeginPlay
  (|CallParentFunction))

(event Collision|EventActorBeginOverlap
  (params (OtherActor :type Actor%20Object%20Reference))
  (|CallParentFunction OtherActor) ; 此节点被禁用，将不会被调用。\n从引脚连出引线来编译功能。
)

(event EventTick
  (params (DeltaSeconds :type Float%20%28single-precision%29))
  (|CallParentFunction DeltaSeconds) ; 此节点被禁用，将不会被调用。\n从引脚连出引线来编译功能。
)

(event EventDestroyed
  (|CallParentFunction))

(event EventUseItem
  (|CallParentFunction))

(fn ConstructionScript
  (|CallParentFunction))

(fn ActivateRadio)

(fn OnRepNumConnected)

(fn ResetAlarm)

(fn SetMaterial
  (params (EnabledFOV :type Boolean))
  (|CallParentFunction EnabledFOV))