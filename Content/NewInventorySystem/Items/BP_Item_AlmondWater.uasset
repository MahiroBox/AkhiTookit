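; Almond Water item for the inventory system, a child Blueprint that leaves its use behavior to the parent class.
; UseItem and the construction script only call the parent versions.
; SetMaterial ignores its EnabledFOV input and always passes false to the parent.
; PlayAnimation, OnEventLoaded and the montage-style callbacks are empty, and BeginPlay, overlap and Tick are disabled placeholders.
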(event Custom|OnNotifyEnd_3881A8424F905F4C29433AB5756CB3DA
  (params (NotifyName :type Name)))

(event Custom|OnNotifyBegin_3881A8424F905F4C29433AB5756CB3DA
  (params (NotifyName :type Name)))

(event Custom|OnInterrupted_3881A8424F905F4C29433AB5756CB3DA
  (params (NotifyName :type Name)))

(event Custom|OnBlendOut_3881A8424F905F4C29433AB5756CB3DA
  (params (NotifyName :type Name)))

(event Custom|OnCompleted_3881A8424F905F4C29433AB5756CB3DA
  (params (NotifyName :type Name)))

(event Custom|PlayAnimation)

(event Custom|OnEventLoaded
  (params (EventType :type Byte)))

(event EventBeginPlay
  (|CallParentFunction) ; 此节点被禁用，将不会被调用。\n从引脚连出引线来编译功能。
)

(event Collision|EventActorBeginOverlap
  (params (OtherActor :type Actor%20Object%20Reference))
  (|CallParentFunction OtherActor) ; 此节点被禁用，将不会被调用。\n从引脚连出引线来编译功能。
)

(event EventTick
  (params (DeltaSeconds :type Float%20%28single-precision%29))
  (|CallParentFunction DeltaSeconds) ; 此节点被禁用，将不会被调用。\n从引脚连出引线来编译功能。
)

(event EventUseItem
  (|CallParentFunction))

(fn ConstructionScript
  (|CallParentFunction))

(fn SetMaterial
  (params (EnabledFOV :type Boolean))
  (|CallParentFunction false))