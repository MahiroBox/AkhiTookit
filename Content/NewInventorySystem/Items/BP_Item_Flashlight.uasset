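; BP_Item_Flashlight is a flashlight item for the inventory system, extending a parent item class whose UseItem it calls.
; It declares events for power toggling, light fading, flicker and animation, alongside several timelines, montage callbacks and an IsFlashlightOn RepNotify.
; These are empty stubs: the radius and intensity helpers return zero, and only BeginPlay and UseItem actively forward to the parent.
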(event Custom|Timeline_0__FinishedFunc)

(event Custom|Timeline_0__UpdateFunc)

(event Custom|OnInterrupted_858C6BED431A8EBEEAB2D09BA256DAA6
  (params (NotifyName :type Name)))

(event Custom|OnBlendOut_858C6BED431A8EBEEAB2D09BA256DAA6
  (params (NotifyName :type Name)))

(event Custom|OnCompleted_858C6BED431A8EBEEAB2D09BA256DAA6
  (params (NotifyName :type Name)))

(event Custom|ToggleFadePower
  (params (FadeOut :type Boolean)))

(event Custom|PlayAnimation)

(event Custom|StartFlicker)

(event Custom|ToggleFlashlightPower
  (params (Power :type Boolean)))

(event Custom|FadeLight
  (params (FadeOut :type Boolean)))

(event Custom|Timeline_1__FinishedFunc)

(event Custom|Timeline_1__UpdateFunc)

(event Custom|TogglePower__FinishedFunc)

(event Custom|TogglePower__UpdateFunc)

(event Custom|Timeline_2__FinishedFunc)

(event Custom|Timeline_2__UpdateFunc)

(event Custom|OnNotifyEnd_858C6BED431A8EBEEAB2D09BA256DAA6
  (params (NotifyName :type Name)))

(event Custom|OnNotifyBegin_858C6BED431A8EBEEAB2D09BA256DAA6
  (params (NotifyName :type Name)))

(event EventBeginPlay
  (|CallParentFunction))

(event Collision|EventActorBeginOverlap
  (params (OtherActor :type Actor%20Object%20Reference))
  (|CallParentFunction OtherActor) ; 此节点被禁用，将不会被调用。\n从引脚连出引线来编译功能。
)

(event EventTick
  (params (DeltaSeconds :type Float%20%28single-precision%29))
  (|CallParentFunction DeltaSeconds) ; 此节点被禁用，将不会被调用。\n从引脚连出引线来编译功能。
)

(event EventUseItem
  (|CallParentFunction))

(fn ConstructionScript
  (|CallParentFunction))

(fn GetAdjustedRadius
  (params (Radius :type Float%20%28single-precision%29))
  (return 0.0))

(fn GetAdjustedIntensity
  (params (Intensity :type Float%20%28single-precision%29))
  (return 0.0))

(fn OnRepIsFlashlighton)