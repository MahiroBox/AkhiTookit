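; Chainsaw item Blueprint in the new inventory system, a thin child that leaves its behavior to the parent class.
; UseItem, Destroyed and the construction script only forward to the parent.
; SetMaterial also calls the parent but always passes false, ignoring its EnabledFOV input.
; PlayAnimation, OC_Trace, the Recoil timeline events and the montage callbacks are empty, and BeginPlay, overlap and Tick are disabled.
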(event Custom|Recoil__FinishedFunc)

(event Custom|Recoil__UpdateFunc)

(event Custom|OnBlendOut_FBCA7ED7436A8ED7C154A2B37E6C3659
  (params (NotifyName :type Name)))

(event Custom|OnCompleted_FBCA7ED7436A8ED7C154A2B37E6C3659
  (params (NotifyName :type Name)))

(event Custom|PlayAnimation)

(event Custom|OC_Trace)

(event Custom|OnNotifyEnd_702F9C624045D5D1016E778DEB923CD4
  (params (NotifyName :type Name)))

(event Custom|OnNotifyBegin_702F9C624045D5D1016E778DEB923CD4
  (params (NotifyName :type Name)))

(event Custom|OnInterrupted_702F9C624045D5D1016E778DEB923CD4
  (params (NotifyName :type Name)))

(event Custom|OnBlendOut_702F9C624045D5D1016E778DEB923CD4
  (params (NotifyName :type Name)))

(event Custom|OnCompleted_702F9C624045D5D1016E778DEB923CD4
  (params (NotifyName :type Name)))

(event Custom|OnNotifyEnd_FBCA7ED7436A8ED7C154A2B37E6C3659
  (params (NotifyName :type Name)))

(event Custom|OnNotifyBegin_FBCA7ED7436A8ED7C154A2B37E6C3659
  (params (NotifyName :type Name)))

(event Custom|OnInterrupted_FBCA7ED7436A8ED7C154A2B37E6C3659
  (params (NotifyName :type Name)))

(event EventBeginPlay
  (|CallParentFunction) ; 此节点被禁用，将不会被调用。\n从引脚连出引线来编译功能。
)

(event Collision|EventActorBeginOverlap
  (params (OtherActor :type Actor%20Object%20Reference))
  (|CallParentFunction OtherActor) ; 此节点被禁用，将不会被调用。\n从引脚连出引线来编译功能。
)

(event EventTick
  (params (DeltaSeconds :type Float%20%28single-precision%29))
  (|CallParentFunction DeltaSeconds) ; 此节点被禁用，将不会被调用。\n从引脚连出引线来编译功能。
)

(event EventUseItem
  (|CallParentFunction))

(event EventDestroyed
  (|CallParentFunction))

(fn ConstructionScript
  (|CallParentFunction))

(fn SetMaterial
  (params (EnabledFOV :type Boolean))
  (|CallParentFunction false))