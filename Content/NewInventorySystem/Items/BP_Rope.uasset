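; BP_Rope is a rope item in the new inventory system, currently a skeleton with no rope logic of its own.
; UseItem, Destroyed and the construction script only call their parent versions, while BeginPlay, overlap and Tick are disabled.
; Montage notify callbacks and throw, trace, show, hide and remove events are empty stubs, with prefixes suggesting multicast, owning-client and server RPCs.
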(event Custom|OnNotifyEnd_6D75097146D9F446056AF481A6C55D82
  (params (NotifyName :type Name)))

(event Custom|OnNotifyBegin_6D75097146D9F446056AF481A6C55D82
  (params (NotifyName :type Name)))

(event Custom|SRV_HideRope)

(event Custom|SRV_ShowRope
  (params (Actor :type Actor%20Object%20Reference) (Location :type Vector)))

(event Custom|RemoveRope)

(event Custom|OnInterrupted_6D75097146D9F446056AF481A6C55D82
  (params (NotifyName :type Name)))

(event Custom|OnBlendOut_6D75097146D9F446056AF481A6C55D82
  (params (NotifyName :type Name)))

(event Custom|OnCompleted_6D75097146D9F446056AF481A6C55D82
  (params (NotifyName :type Name)))

(event Custom|MC_Throw)

(event Custom|OC_HideRope)

(event Custom|OC_Trace)

(event Custom|OC_ShowRope
  (params (Actor :type Actor%20Object%20Reference) (Location :type Vector)))

(event EventBeginPlay
  (|CallParentFunction) ; 此节点被禁用，将不会被调用。\n从引脚连出引线来编译功能。
)

(event Collision|EventActorBeginOverlap
  (params (OtherActor :type Actor%20Object%20Reference))
  (|CallParentFunction OtherActor) ; 此节点被禁用，将不会被调用。\n从引脚连出引线来编译功能。
)

(event EventTick
  (params (DeltaSeconds :type Float%20%28single-precision%29))
  (|CallParentFunction DeltaSeconds) ; 此节点被禁用，将不会被调用。\n从引脚连出引线来编译功能。
)

(event EventUseItem
  (|CallParentFunction))

(event EventDestroyed
  (|CallParentFunction))

(fn ConstructionScript
  (|CallParentFunction))