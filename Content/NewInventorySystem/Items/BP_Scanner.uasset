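; BP_Scanner is a scanner item Blueprint in the new inventory system, outlining LiDAR, wave scan and motion scanner modes.
; BeginPlay, Tick, UseItem, construction and SetMaterial only forward to the parent class.
; Mode toggles, replication callbacks, fire and LiDAR events, and trace, UV-fix, targeting and sound functions are empty stubs or return defaults, so this graph implements no scanning logic itself.
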(event Custom|SetEnableLiDAR
  (params (Enable :type Boolean)))

(event Custom|SetEnableWaveScan
  (params (bEnable :type Boolean)))

(event Custom|SetEnableMotionScanner
  (params (bEnable :type Boolean)))

(event Custom|SetScanDistance
  (params (NewDistance :type Float%20%28single-precision%29)))

(event Custom|SpawnScannerBeam
  (params (BeamStart :type Vector) (BeamEnd :type Vector)))

(event Custom|ResetSKCollisionUVBool)

(event Custom|MC_Fire)

(event Custom|Initialize)

(event Custom|OC_Fire)

(event Custom|SRV_Lidar
  (params (HitResult :type Hit%20Result%20Structure) (Color :type Color%20Structure)))

(event EventBeginPlay
  (|CallParentFunction))

(event Collision|EventActorBeginOverlap
  (params (OtherActor :type Actor%20Object%20Reference))
  (|CallParentFunction OtherActor) ; 此节点被禁用，将不会被调用。\n从引脚连出引线来编译功能。
)

(event EventTick
  (params (DeltaSeconds :type Float%20%28single-precision%29))
  (|CallParentFunction DeltaSeconds))

(event EventUseItem
  (|CallParentFunction))

(fn ConstructionScript
  (|CallParentFunction))

(fn SetMaterial
  (params (EnabledFOV :type Boolean))
  (|CallParentFunction EnabledFOV))

(fn GetMaterial
  (params (Material :type Material%20Interface%20Object%20Reference))
  (return 0))

(fn LiDAR
  (params (Delta :type Float%20%28single-precision%29%20%28by%20ref%29)))

(fn InitializeColors)

(fn InitializeMaterials)

(fn FixUVStretching
  (params (HitLocation :type Vector) (HitNormal :type Vector) (HitComponent :type Primitive%20Component%20Object%20Reference) (FaceIndex :type Integer) (HitUVLocation :type Vector%202D%20Structure))
  (return 0.0 "0, 0, 0"))

(fn ScannerTraceCalc
  (return "0, 0, 0" "0, 0, 0"))

(fn SetTargetPosition
  (params (OneTarget :type Boolean) (SetMotionScanner :type %20Object%20Reference) (SetNpcMesh :type Static%20Mesh%20Component%20Object%20Reference)))

(fn UpdateScanPercent)

(fn UpdateMinDistance
  (return 0.0))

(fn UpdateTargetSound
  (params (InFloat :type Float%20%28single-precision%29) (bEnable :type Boolean)))

(fn SetTargets)

(fn SetNewPositionTarget
  (params (SecondLocation :type Vector))
  (return "0, 0, 0"))

(fn OnRepBIsLiDAREnable)

(fn OnRepBIsWaveScannerEnbale)

(fn OnRepBIsMotionScannerEnable)

(fn SoundChangeDistance
  (params (NewDistance :type Float%20%28single-precision%29%20%28by%20ref%29)))

(fn SetStartEnableMotionScanner
  (params (Activate :type Boolean)))