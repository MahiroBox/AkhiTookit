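; BP_Item_Glowstick is the glowstick item Blueprint in the new inventory system, currently mostly a skeleton over its parent class.
; BeginPlay, Tick, UseItem and the construction script only forward to the parent.
; Montage callbacks, MC_Fire and MC_PlaySubtitle are empty.
; GetAdjustedRadius and GetAdjustedIntensity ignore their inputs and return zero.
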(event Custom|OnNotifyEnd_AE195271461F08CE34117A8A70C47D64
  (params (NotifyName :type Name)))

(event Custom|OnNotifyBegin_AE195271461F08CE34117A8A70C47D64
  (params (NotifyName :type Name)))

(event Custom|OnInterrupted_AE195271461F08CE34117A8A70C47D64
  (params (NotifyName :type Name)))

(event Custom|OnBlendOut_AE195271461F08CE34117A8A70C47D64
  (params (NotifyName :type Name)))

(event Custom|OnCompleted_AE195271461F08CE34117A8A70C47D64
  (params (NotifyName :type Name)))

(event Custom|MC_Fire)

(event Custom|MC_PlaySubtitle)

(event EventBeginPlay
  (|CallParentFunction))

(event Collision|EventActorBeginOverlap
  (params (OtherActor :type Actor%20Object%20Reference))
  (|CallParentFunction OtherActor) ; 此节点被禁用，将不会被调用。\n从引脚连出引线来编译功能。
)

(event EventTick
  (params (DeltaSeconds :type Float%20%28single-precision%29))
  (|CallParentFunction DeltaSeconds))

(event EventUseItem
  (|CallParentFunction))

(fn ConstructionScript
  (|CallParentFunction))

(fn GetAdjustedRadius
  (params (Radius :type Float%20%28single-precision%29))
  (return 0.0))

(fn GetAdjustedIntensity
  (params (Intensity :type Float%20%28single-precision%29))
  (return 0.0))