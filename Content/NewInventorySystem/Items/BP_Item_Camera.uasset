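; Camera inventory item Blueprint, outlining picture snapping, a flash timeline, photo switching and a toggleable light.
; Its server, multicast and RepNotify names suggest networked photo and flashlight state, but these handlers, the timeline and the montage callbacks are empty stubs.
; BeginPlay, Tick, UseItem and construction only call the parent, and the overlap event is disabled.
; SetMaterial ignores its EnabledFOV input and always passes false to the parent.
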(event Custom|Flash__FinishedFunc)

(event Custom|Flash__UpdateFunc)

(event Custom|OnInterrupted_E8F7DC85419A58268AB58B8CC984D2BD
  (params (NotifyName :type Name)))

(event Custom|OnBlendOut_E8F7DC85419A58268AB58B8CC984D2BD
  (params (NotifyName :type Name)))

(event Custom|OnCompleted_E8F7DC85419A58268AB58B8CC984D2BD
  (params (NotifyName :type Name)))

(event Custom|OnNotifyEnd_49041A0D437647D77BE07E918FD7721C
  (params (NotifyName :type Name)))

(event Custom|OnNotifyBegin_49041A0D437647D77BE07E918FD7721C
  (params (NotifyName :type Name)))

(event Custom|OnInterrupted_49041A0D437647D77BE07E918FD7721C
  (params (NotifyName :type Name)))

(event Custom|OnBlendOut_49041A0D437647D77BE07E918FD7721C
  (params (NotifyName :type Name)))

(event Custom|OnCompleted_49041A0D437647D77BE07E918FD7721C
  (params (NotifyName :type Name)))

(event Custom|SnapPicture)

(event Custom|Update)

(event Custom|Flash__Snap__EventFunc)

(event Custom|StopPicture)

(event Custom|MC_SwitchPhotos)

(event Custom|PlayAnimation)

(event Custom|SRV_ToggleLight
  (params (Enabled :type Boolean)))

(event Custom|OnNotifyEnd_3ABC687248F18F6E8E9F69BF9EB015A7
  (params (NotifyName :type Name)))

(event Custom|OnNotifyBegin_3ABC687248F18F6E8E9F69BF9EB015A7
  (params (NotifyName :type Name)))

(event Custom|OnInterrupted_3ABC687248F18F6E8E9F69BF9EB015A7
  (params (NotifyName :type Name)))

(event Custom|OnBlendOut_3ABC687248F18F6E8E9F69BF9EB015A7
  (params (NotifyName :type Name)))

(event Custom|OnCompleted_3ABC687248F18F6E8E9F69BF9EB015A7
  (params (NotifyName :type Name)))

(event Custom|OnNotifyEnd_E8F7DC85419A58268AB58B8CC984D2BD
  (params (NotifyName :type Name)))

(event Custom|OnNotifyBegin_E8F7DC85419A58268AB58B8CC984D2BD
  (params (NotifyName :type Name)))

(event EventBeginPlay
  (|CallParentFunction))

(event Collision|EventActorBeginOverlap
  (params (OtherActor :type Actor%20Object%20Reference))
  (|CallParentFunction OtherActor) ; 此节点被禁用，将不会被调用。\n从引脚连出引线来编译功能。
)

(event EventTick
  (params (DeltaSeconds :type Float%20%28single-precision%29))
  (|CallParentFunction DeltaSeconds))

(event EventUseItem
  (|CallParentFunction))

(fn ConstructionScript
  (|CallParentFunction))

(fn OnRepIsFlashlighton)

(fn OnRepCurrentPicture)

(fn SetMaterial
  (params (EnabledFOV :type Boolean))
  (|CallParentFunction false))